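; BP_TempWaypointActor is a placed waypoint actor, apparently temporary, that displays a marker widget while the local player is nearby.
; On BeginPlay it passes its world location to the BP_WaypointMarker inside the MarkerWidget component as the origin (variable spelled OiriginLocation).
; Box overlap events show the widget when player 0's controlled pawn enters and hide it when that pawn leaves.
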(event `self.ReceiveBeginPlay`
  (bind _asbp_waypoint_marker (cast `/Game/UI/WaypointMarker/BP_WaypointMarker` (`WidgetComponent.GetUserWidgetObject` (`self.MarkerWidget`))))
  (set `/Game/UI/WaypointMarker/BP_WaypointMarker.OiriginLocation` (`self.K2_GetActorLocation`) _asbp_waypoint_marker))

(event `self.Box.OnComponentBeginOverlap`
  (params (OverlappedComponent :type "PrimitiveComponent Object Reference") (OtherActor :type "Actor Object Reference") (OtherComp :type "PrimitiveComponent Object Reference") (OtherBodyIndex :type Integer) (bFromSweep :type Boolean) (SweepResult :type "HitResult Structure (by ref)"))
  (if (== OtherActor (`Controller.K2_GetPawn` (`PlayerState.GetPlayerController` (`GameplayStatics.GetPlayerState` 0))))
    (`SceneComponent.SetVisibility` (`self.MarkerWidget`) true false)))

(event `self.Box.OnComponentEndOverlap`
  (params (OverlappedComponent :type "PrimitiveComponent Object Reference") (OtherActor :type "Actor Object Reference") (OtherComp :type "PrimitiveComponent Object Reference") (OtherBodyIndex :type Integer))
  (if (== (`Controller.K2_GetPawn` (`PlayerState.GetPlayerController` (`GameplayStatics.GetPlayerState` 0))) OtherActor)
    (`SceneComponent.SetVisibility` (`self.MarkerWidget`) false false)))

(fn `UserConstructionScript`)