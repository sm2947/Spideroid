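; Hackable component that runs a one-time response when an object is hacked.
; HackDone_Event guards on the Hacked flag, then optionally plays a 2D sound and waits a configurable delay.
; If waypoints are enabled, it then unhides every actor in the Waypoints array, with debug prints along the way.
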(event `HackDone_Event`
  (if (not (`self.hacked`))
    (set `self.hacked` true)
    (`KismetSystemLibrary.PrintString` "Hackable event triggered")
    (if (`self.HasSoundAfterHack`)
      (`GameplayStatics.PlaySound2D` (`self.PlayAfterHack`) 1.0 1.0 0.0 null null)
      (`KismetSystemLibrary.Delay` (`self.Delay`))
      (`KismetSystemLibrary.PrintString` "Delay done"))
    (if (`self.HasWaypoint`)
      (for _array_element (`self.Waypoints`)
        (`Actor.SetActorHiddenInGame` _array_element false)))))