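; Archived enemy pawn Blueprint with waypoint patrol, player detection and a rough chase event.
; Patrol moves through PatrolPoints with AIMoveTo, re-calling itself after a short delay and wrapping at MaxPoint.
; PawnSensing hands the spotted player to AIC_Enemy's attack state.
; ChasePlayer sets FlyingAI's homing target to the Spidership capsule, then immediately destroys the player; BeginPlay and the DetectBox overlap do nothing effective.
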(event `self.ReceiveBeginPlay`)

(event `Patrol`
  (bind _locations (`self.Locations`))
  (`|AIMoveTo` self (`|GetArrayItem` (`self.PatrolPoints`) (`self.Locations`)) null
    (:`then`
      (`KismetSystemLibrary.PrintText` "5!" true true (struct :`R` 1.0 :`A` 1.0) 3.0)
      (`KismetSystemLibrary.Delay` 0.2)
      (bind _result (`/Engine/EditorBlueprintResources/StandardMacros.IncrementInt` _locations)
        (:`  `
          (set `self.Locations` _result)
          (if (== _locations (`self.MaxPoint`))
            (set `self.Locations` 0))
          (`self.Patrol`))))))

(event `ChasePlayer`
  (bind _returnvalue (`GameplayStatics.GetPlayerCharacter` 0))
  ;[1 1 1] ChaseAttack
  (set `ProjectileMovementComponent.HomingTargetComponent` (`Character.CapsuleComponent` (cast `/Game/ThirdPerson/Blueprints/Spidership` (`GameplayStatics.GetPlayerCharacter` 0) :!pure true)) (`self.FlyingAI`))
  (`self.K2_DestroyActor` _returnvalue)
  (`KismetSystemLibrary.PrintString` (`KismetSystemLibrary.GetDisplayName` _returnvalue))
  (`KismetSystemLibrary.PrintString` "Destroy actor called"))

(event `self.PawnSensing.OnSeePawn`
  (params (Pawn :type "Pawn Object Reference"))
  ;[1 1 1] Detection
  (`KismetSystemLibrary.PrintText` "You have been spotted!" true true (struct :`R` 1.0 :`A` 1.0) 3.0)
  (`GameplayStatics.GetAllActorsOfClass` "/Game/Blueprints/AI/BP_EnemyPawn.BP_EnemyPawn_C")
  (bind _asaic_enemy (cast `/Game/Blueprints/AI/AIC_Enemy` (`AIBlueprintHelperLibrary.GetAIController` null)))
  (`/Game/Blueprints/AI/AIC_Enemy.SetStateasAttack` _asaic_enemy (`GameplayStatics.GetPlayerCharacter` 0)))

(event `self.DetectBox.OnComponentBeginOverlap`
  (params (OverlappedComponent :type "PrimitiveComponent Object Reference") (OtherActor :type "Actor Object Reference") (OtherComp :type "PrimitiveComponent Object Reference") (OtherBodyIndex :type Integer) (bFromSweep :type Boolean) (SweepResult :type "HitResult Structure (by ref)"))
  (cast `PlayerController` OtherActor))

(fn `UserConstructionScript`)