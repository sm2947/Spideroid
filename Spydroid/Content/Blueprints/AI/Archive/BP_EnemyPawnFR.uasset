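; Flying enemy pawn that patrols waypoints and fires on the player Spidership when detected, with debug prints throughout.
; Tick cycles patrol points, nudging rotation toward the next and retargeting the FlyingAI homing component after a delay.
; DetectBox overlap with an unghosted player starts a cooldown-gated firing loop, choosing between two bullet spawns by relative height.
; AttackBox exit requests AIC_Enemy's patrol state; ChasePlayer homes on, then destroys, the player.
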(event `self.ReceiveBeginPlay`
  (`KismetSystemLibrary.Delay` 0.2)
  (bind _outactors (`GameplayStatics.GetAllActorsWithTag` "Player"))
  (bind _asspidership (cast `/Game/ThirdPerson/Blueprints/Spidership` (`|GetArrayItem` _outactors)))
  (set `self.Target_0` _asspidership)
  (`KismetSystemLibrary.PrintString` "Cast succeeded"))

(event `self.ReceiveTick`
  (params (DeltaSeconds :type "Float (single-precision)"))
  (bind _locations (`self.Locations`))
  (if (== (`self.K2_GetActorLocation`) (`self.K2_GetActorLocation` (`|GetArrayItem` (`self.Patrolpoint`) (`self.Locations`))) :`ErrorTolerance` 15000.0)
    (bind _result (`/Engine/EditorBlueprintResources/StandardMacros.IncrementInt` _locations)
      (:`  `
        (set `self.Locations` _result)
        (`KismetSystemLibrary.PrintText` (`KismetTextLibrary.Conv_IntToText` _locations))
        (if (== _locations (`self.MaxPoint`))
          (set `self.Locations` 0))
        (`self.Patrol`)))))

(event `self.PawnSensing.OnSeePawn`
  (params (Pawn :type "Pawn Object Reference")))

(event `Patrol`
  (`self.Turn`)
  (`KismetSystemLibrary.Delay` 3.0)
  (set `ProjectileMovementComponent.HomingTargetComponent` (`Character.CapsuleComponent` (`|GetArrayItem` (`self.Patrolpoint`) (`self.Locations`))) (`self.FlyingAI`))
  (`KismetSystemLibrary.PrintText` "6!" true true (struct :`R` 1.0 :`A` 1.0) 3.0))

(event `Turn`
  (`self.K2_SetActorRotation` (`KismetMathLibrary.RInterpTo_Constant` (`self.K2_GetActorRotation`) (`KismetMathLibrary.FindLookAtRotation` (`self.K2_GetActorLocation`) (`self.K2_GetActorLocation` (`|GetArrayItem` (`self.Patrolpoint`) (`self.Locations`)))) (`GameplayStatics.GetWorldDeltaSeconds`) 0.5)))

(event `ChasePlayer`
  (bind _returnvalue (`GameplayStatics.GetPlayerCharacter` 0))
  ;[1 1 1] ChaseAttack
  (set `ProjectileMovementComponent.HomingTargetComponent` (`Character.CapsuleComponent` (cast `/Game/ThirdPerson/Blueprints/Spidership` (`GameplayStatics.GetPlayerCharacter` 0) :!pure true)) (`self.FlyingAI`))
  (`self.K2_DestroyActor` _returnvalue)
  (`KismetSystemLibrary.PrintString` (`KismetSystemLibrary.GetDisplayName` _returnvalue))
  (`KismetSystemLibrary.PrintString` "Destroy actor called"))

(event `self.DetectBox.OnComponentBeginOverlap`
  (params (OverlappedComponent :type "PrimitiveComponent Object Reference") (OtherActor :type "Actor Object Reference") (OtherComp :type "PrimitiveComponent Object Reference") (OtherBodyIndex :type Integer) (bFromSweep :type Boolean) (SweepResult :type "HitResult Structure (by ref)"))
  (bind _returnvalue (== OtherActor (`self.Target_0`)))
  (`KismetSystemLibrary.PrintString` (`KismetSystemLibrary.GetDisplayName` OtherActor))
  (`KismetSystemLibrary.PrintString` (`KismetStringLibrary.Conv_BoolToString` _returnvalue))
  (if _returnvalue
    (if (`/Game/ThirdPerson/Blueprints/Spidership.IsGhosted` (`self.Target_0`))
      (`KismetSystemLibrary.PrintString` "Player Ghosted!")
      (else
        (`KismetSystemLibrary.PrintText` "You have been spotted!" true true (struct :`R` 1.0 :`A` 1.0) 3.0)
        (`self.Shoot Player`)))))

(event `Shoot Player`
  (bind (_returnvalue_x _returnvalue_y _returnvalue_z) (`KismetMathLibrary.BreakVector` (`self.K2_GetActorLocation` self)))
  (`KismetSystemLibrary.PrintString` "Shoot player called")
  (if (`self.shootready`) :!label _label
    (bind (_returnvalue_x_2 _returnvalue_y_2 _returnvalue_z_2) (`KismetMathLibrary.BreakVector` (`self.K2_GetActorLocation` (stale `self.DetectBox.OnComponentBeginOverlap` OtherActor))))
    (if (>= _returnvalue_z_2 _returnvalue_z)
      (bind _returnvalue (`|SpawnActorFromClass` "/Game/Blueprints/AI/BP_ProjectileBullet.BP_ProjectileBullet_C" (`SceneComponent.K2_GetComponentToWorld` (`self.BulletSpawn`)) "Undefined" "MultiplyWithRoot" null null))
      (else
        (`|SpawnActorFromClass` "/Game/Blueprints/AI/BP_ProjectileBullet.BP_ProjectileBullet_C" (`SceneComponent.K2_GetComponentToWorld` (`self.BulletSpawn1`)) "Undefined" "MultiplyWithRoot" null null)))
    (`PrimitiveComponent.IgnoreActorWhenMoving` (`self.StaticMesh`) _returnvalue false)
    (if (not (`/Game/ThirdPerson/Blueprints/Spidership.IsGhosted` (`self.Target_0`)))
      (set `self.shootready` false)
      (`KismetSystemLibrary.Delay` 2.0)
      (set `self.shootready` true)
      (goto _label))))

(event `self.AttackBox.OnComponentEndOverlap`
  (params (OverlappedComponent :type "PrimitiveComponent Object Reference") (OtherActor :type "Actor Object Reference") (OtherComp :type "PrimitiveComponent Object Reference") (OtherBodyIndex :type Integer))
  (cast `PlayerController` OtherActor)
  (`KismetSystemLibrary.PrintText` "You have escaped!" true true (struct :`R` 1.0 :`A` 1.0) 3.0)
  (bind _asaic_enemy (cast `/Game/Blueprints/AI/AIC_Enemy` (`AIBlueprintHelperLibrary.GetAIController` null)))
  (`/Game/Blueprints/AI/AIC_Enemy.SetStateasPatrol` _asaic_enemy))

(fn `UserConstructionScript`)