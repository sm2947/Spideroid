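; AI controller for an enemy that runs the FlyingAIBT behavior tree shortly after possession, then starts it in the patrol state.
; SetStateasPatrol and SetStateasAttack switch the blackboard's E_AIState key, with the attack version also storing the target.
; Possession also prints a red "!" debug message.
; Disconnected leftover nodes, including patrol point A/B writes and an attack call, never execute.
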(event `self.ReceivePossess`
  (params (PossessedPawn :type "Pawn Object Reference"))
  (`KismetSystemLibrary.PrintText` "!" true true (struct :`R` 1.0 :`A` 1.0) 3.0)
  (`KismetSystemLibrary.Delay` 0.2)
  (`self.RunBehaviorTree` "/Game/Blueprints/AI/FlyingAIBT.FlyingAIBT")
  (`self.SetStateasPatrol`))

(fn `SetStateasAttack`
  (params (AttackTarget :type "Actor Object Reference"))
  (`BlackboardComponent.SetValueAsObject` (`self.Blackboard`) (`self.Attack Target Key Name`) AttackTarget)
  (`BlackboardComponent.SetValueAsEnum` (`self.Blackboard`) (`self.State Key Name`) (enumliteral `/Game/Blueprints/AI/E_AIState` "NewEnumerator1")))

(fn `SetStateasPatrol`
  (`BlackboardComponent.SetValueAsEnum` (`self.Blackboard`) (`self.State Key Name`) (enumliteral `/Game/Blueprints/AI/E_AIState` "NewEnumerator0")))

(fn `UserConstructionScript`)