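; Projectile bullet, filed under AI, that takes the player as its homing target.
; On BeginPlay it finds the first actor tagged Player, casts it to Character and sets its capsule as the ProjectileMovement homing target.
; It destroys itself on a collision hit or after a short delay, with debug prints and no damage logic.
; If the Character cast fails, the timed destroy never starts.
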(event `self.ReceiveBeginPlay`
  (bind _outactors (`GameplayStatics.GetAllActorsWithTag` "Player"))
  (bind _ascharacter (cast `Character` (`|GetArrayItem` _outactors)))
  (set `ProjectileMovementComponent.HomingTargetComponent` (`Character.CapsuleComponent` _ascharacter) (`self.ProjectileMovement`))
  (`KismetSystemLibrary.PrintString` "Projectile Launched")
  (`KismetSystemLibrary.Delay` 3.0)
  (`self.K2_DestroyActor`)
  (`KismetSystemLibrary.PrintString` "Projectile destroyed"))

(event `self.Collisiion.OnComponentHit`
  (params (HitComponent :type "PrimitiveComponent Object Reference") (OtherActor :type "Actor Object Reference") (OtherComp :type "PrimitiveComponent Object Reference") (NormalImpulse :type "Vector Structure") (Hit :type "HitResult Structure (by ref)"))
  (`self.K2_DestroyActor`)
  (`KismetSystemLibrary.PrintString` "Projectile hit"))

(fn `UserConstructionScript`)